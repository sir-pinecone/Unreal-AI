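; Base class for toxic food items that harm the actor using them, built on a parent usable-item class.
; BeginPlay sets StatValue to a negative amount.
; UseItem checks that the actor is valid, applies DamageToApply to it, activates the Explosion component, then runs the parent's use logic.
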(event `self.ReceiveBeginPlay`
  (set `self.StatValue` -100.0))

(event `self.UseItem`
  (params (Actor :type "Actor Object Reference"))
  (`/Engine/EditorBlueprintResources/StandardMacros.IsValid` Actor
    (:`Is Valid`
      (`GameplayStatics.ApplyDamage` Actor (`self.DamageToApply`) null self)
      (`ActorComponent.Activate` (`self.Explosion`) false)
      (`parent.UseItem` Actor))))

(fn `UserConstructionScript`
  (`parent.UserConstructionScript`))