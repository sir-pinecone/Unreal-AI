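; Player controller that drives a stored pawn with axis movement and mouse-controlled rotation, distinguishing mouse clicks from holds.
; Both movement inputs share one path that offsets the pawn horizontally relative to control rotation and aligns its arrow.
; Tick-fed gates time each button against a short hold threshold.
; Holding right rotates control yaw and the pawn's spring arm; left input and right clicks only print debug messages.
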(event `InputAxis|MoveForward`
  (params (AxisValue :type "Float (single-precision)"))
  (bind _returnvalue (`self.GetControlRotation`))
  ;[0 1 0.5882] Movement
  (`self.K2_AddActorLocalOffset` (`self.StoredPawn`) (* (* (+ (* (`KismetMathLibrary.GetForwardVector` _returnvalue) AxisValue) (* (`KismetMathLibrary.GetRightVector` _returnvalue) (stale `InputAxis|MoveRight` AxisValue))) (`self.MovementRate`)) (1.0 1.0 0.0)) false false :!label _label)
  (`SceneComponent.K2_SetWorldRotation` (`/Game/AI/AI_PlayerPawn_BP.ControllerArrow` (`self.StoredPawn`)) (`self.GetControlRotation`) false false))

(event `InputAxis|MoveRight`
  (params (AxisValue :type "Float (single-precision)"))
  ;[0 1 0.5882] Movement
  (goto _label))

(event `Key|LeftMouseButton`
  (params (Key :type "Key Structure" :default "AnyKey"))
  (bind _leftclickholdcounter (`self.LeftClickHoldCounter`))
  ;[0 0.8752 1] Left and right mouse interactions
  (:`Pressed`
    (goto _label_2 :!via `Open`))
  (:`Released`
    (if (not (not (`self.bLeftClick`)))
      (`KismetSystemLibrary.PrintString` "*** Left Click Detected ***"))
    (set `self.LeftClickHoldCounter` 0.0)
    (set `self.bLeftClick` true)
    (goto _label_2 :!via `Close`)))

(event `self.ReceiveTick`
  (params (DeltaSeconds :type "Float (single-precision)"))
  (bind _rightclickholdcounter (`self.RightClickHoldCounter`))
  (bind _leftclickholdcounter (`self.LeftClickHoldCounter`))
  (bind _springarm (`/Game/AI/AI_PlayerPawn_BP.SpringArm` (`self.StoredPawn`)))
  ;[0 0.8752 1] Left and right mouse interactions
  (`|ExecutionSequence`
    (:`then_0`
      (`/Engine/EditorBlueprintResources/StandardMacros.Gate` true :!label _label_2
        (:`Exit`
          (if (`self.bLeftClick`)
            (if (>= _leftclickholdcounter 0.18)
              (set `self.bLeftClick` false)
              (else
                (set `self.LeftClickHoldCounter` (+ DeltaSeconds _leftclickholdcounter))))
            (else
              (`KismetSystemLibrary.PrintString` "*** Left Mouse Held ***"))))))
    (:`then_1`
      (`/Engine/EditorBlueprintResources/StandardMacros.Gate` true :!label _label_3
        (:`Exit`
          (if (`self.bRightClick`)
            (if (>= _rightclickholdcounter 0.18)
              (set `self.bRightClick` false)
              (else
                (set `self.RightClickHoldCounter` (+ DeltaSeconds _rightclickholdcounter))))
            (else
              (`self.SetControlRotation` (`KismetMathLibrary.MakeRotator` 0.0 0.0 (+ (`self.GetInputAxisKeyValue`) (.yaw (`self.GetControlRotation`)))))
              (`SceneComponent.K2_SetWorldRotation` _springarm (`KismetMathLibrary.MakeRotator` 0.0 (+ (`self.GetInputAxisKeyValue`) (.pitch (`SceneComponent.K2_GetComponentRotation` _springarm))) (+ (`self.GetInputAxisKeyValue`) (.yaw (`SceneComponent.K2_GetComponentRotation` _springarm)))) false false))))))))

(event `Key|RightMouseButton`
  (params (Key :type "Key Structure" :default "AnyKey"))
  ;[0 0.8752 1] Left and right mouse interactions
  (:`Pressed`
    (goto _label_3 :!via `Open`))
  (:`Released`
    (if (not (not (`self.bRightClick`)))
      (`KismetSystemLibrary.PrintString` "*** Right Click Detected ***"))
    (set `self.RightClickHoldCounter` 0.0)
    (set `self.bRightClick` true)
    (goto _label_3 :!via `Close`)))

(fn `UserConstructionScript`)